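; Game player controller that adds the player UI for local players and handles turning the player into an alien.
; InfectionEvent waits briefly, then Infection spawns BP_AlienTest at player 0's pawn transform and possesses it.
; It then calls DestroyActor on GetPlayerPawn(0), re-queried after possession, and removes all widgets.
; GetInfection and GetResearchData are stubs returning constant defaults.
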(event EventBeginPlay
  (if (Pawn|IsLocalPlayerController)
    (bind _returnvalue (UserInterface|CreateWidget "/Game/UI/WB_PlayerUI.WB_PlayerUI_C"))
    (UserInterface|Viewport|AddtoViewport _returnvalue 0)))

(event EventInfectionEvent
  (Utilities|FlowControl|Delay 3.0)
  (CallFunction|Infection))

(fn ConstructionScript)

(fn Infection
  (bind _returnvalue (Game|Player|GetPlayerPawn 0))
  (bind _returnvalue_2 (Game|SpawnActorfromClass "/Game/Blueprints/Characters/BP_AlienTest.BP_AlienTest_C" (Transformation|GetActorTransform _returnvalue) "AdjustIfPossibleButAlwaysSpawn" "MultiplyWithRoot" _returnvalue 0))
  (Pawn|Possess _returnvalue_2)
  (Input|EnableInput _returnvalue_2 self)
  (Actor|DestroyActor (Game|Player|GetPlayerPawn 0))
  (Viewport|RemoveAllWidgets))

(fn GetInfection
  (return false))

(fn GetResearchData
  (return 0))