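; Interactable lever that toggles the lock status of a door and a sign belonging to its room.
; A box overlap shows an interact prompt with the room's lever name to the player.
; Interact relays the toggle through RPC events to a flip-flopped timeline that pitches the pivot.
; After a delay, it updates the first BP_SMDoor1 and BP_Signs whose tags match the room tag.
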(event OnComponentBeginOverlap(Box)
  (params (OverlappedComponent :type Primitive%20Component%20Object%20Reference) (OtherActor :type Actor%20Object%20Reference) (OtherComp :type Primitive%20Component%20Object%20Reference) (OtherBodyIndex :type Integer) (bFromSweep :type Boolean) (SweepResult :type Hit%20Result%20Structure%20%28by%20ref%29))
  (bind _interactprompt (Variables|Default|GetInteractPrompt))
  (if (== OtherActor (Game|GetPlayerCharacter 0))
    (UserInterface|Viewport|AddtoViewport _interactprompt 0)
    (Rendering|Components|TextRender|SetText (Variables|/Game/UI/WB_InteractPrompt.WB_InteractPrompt_C|GetStatusText _interactprompt) (Utilities|Text|ToText(Name) (.LeverName (CallFunction|GetRoomDetails (Variables|Default|GetRoom%20Tag%20In)))))))

(event OnComponentEndOverlap(Box)
  (params (OverlappedComponent :type Primitive%20Component%20Object%20Reference) (OtherActor :type Actor%20Object%20Reference) (OtherComp :type Primitive%20Component%20Object%20Reference) (OtherBodyIndex :type Integer))
  (if (== (Game|GetPlayerCharacter 0) OtherActor)
    (Widget|RemovefromParent (Variables|Default|GetInteractPrompt))))

(event Custom|ToggleLever
  (CallFunction|RPCServerToggleLever))

(event Custom|RPC_ToggleLever
  (Utilities|FlowControl|FlipFlop
    (:A
      (bind _newtrack_0 (Timeline|LeverTime Play)
        (:Update
          (Transformation|SetRelativeRotation (Variables|Default|GetPivotpoint) (Math|Rotator|MakeRotator 0.0 (Math|Float|Lerp 8e+01 -9e+01 _newtrack_0) 0.0) false false))))
    (:B
      (Timeline|LeverTime Reverse))))

(event Custom|RPC_ServerToggleLever
  (CallFunction|RPCToggleLever))

(event EventBeginPlay
  (bind _returnvalue (UserInterface|CreateWidget "/Game/UI/WB_InteractPrompt.WB_InteractPrompt_C"))
  (Variables|Default|SetInteractPrompt _returnvalue))

(event EventInteract
  (params (Player :type Character%20Object%20Reference))
  (bind _room_tag_in (Variables|Default|GetRoom%20Tag%20In))
  (bind _roomtag (CallFunction|GetRoomDetails _room_tag_in))
  (CallFunction|ToggleLever)
  (Utilities|FlowControl|Delay 2.0)
  (Utilities|FlowControl|Sequence
    (:then_0
      (bind _outactors (Actor|GetAllActorsOfClass "/Game/Blueprints/Interactables/BP_SMDoor1.BP_SMDoor1_C"))
      (bind _array_element (Utilities|Array|ForEachLoopwithBreak _outactors :!label _label)
        (:LoopBody
          (if (== (Variables|/Game/Blueprints/Interactables/BP_SMDoor1.BP_SMDoor1_C|GetDoorTag _array_element) _roomtag)
            (Default|SetLockStatus _array_element)
            (goto _label Break)))))
    (:then_1
      (bind _outactors_2 (Actor|GetAllActorsOfClass "/Game/Blueprints/Interactables/BP_Signs.BP_Signs_C"))
      (bind _array_element_2 (Utilities|Array|ForEachLoopwithBreak _outactors_2 :!label _label_2)
        (:LoopBody
          (if (== _roomtag (Variables|/Game/Blueprints/Interactables/BP_Signs.BP_Signs_C|GetSignTag _array_element_2))
            (Default|SetLockStatus _array_element_2)
            (goto _label_2 Break)))))))

(fn ConstructionScript)