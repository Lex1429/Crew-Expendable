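; BP_MapTable is an interactable map table that shows an interact prompt while the local player character overlaps its box.
; Interact calls RPC_ServerOpenMap, which relays to RPC_OpenMap.
; A FlipFlop there alternately creates and shows WB_MapScreen with the mouse cursor, or removes it.
; Closing leaves the cursor visible, and the input-mode nodes are unconnected.
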(event OnComponentBeginOverlap(Box)
  (params (OverlappedComponent :type Primitive%20Component%20Object%20Reference) (OtherActor :type Actor%20Object%20Reference) (OtherComp :type Primitive%20Component%20Object%20Reference) (OtherBodyIndex :type Integer) (bFromSweep :type Boolean) (SweepResult :type Hit%20Result%20Structure%20%28by%20ref%29))
  (if (== OtherActor (Game|GetPlayerCharacter 0))
    (UserInterface|Viewport|AddtoViewport (Variables|Default|GetInteractPrompt) 0)))

(event OnComponentEndOverlap(Box)
  (params (OverlappedComponent :type Primitive%20Component%20Object%20Reference) (OtherActor :type Actor%20Object%20Reference) (OtherComp :type Primitive%20Component%20Object%20Reference) (OtherBodyIndex :type Integer))
  (if (== (Game|GetPlayerCharacter 0) OtherActor)
    (Widget|RemovefromParent (Variables|Default|GetInteractPrompt))))

(event Custom|RPC_OpenMap
  (Utilities|FlowControl|FlipFlop
    (:A
      (bind _returnvalue (UserInterface|CreateWidget "/Game/Map/WB_MapScreen.WB_MapScreen_C"))
      (bind _output_get (Variables|Default|SetMapViewRef _returnvalue))
      (UserInterface|Viewport|AddtoViewport _output_get 0)
      (Variables|/Script/Engine.PlayerController|SetbShowMouseCursor (Game|GetPlayerController 0) true))
    (:B
      (Widget|RemovefromParent (Variables|Default|GetMapViewRef)))))

(event Custom|RPC_ServerOpenMap
  (CallFunction|RPCOpenMap))

(event EventBeginPlay
  (bind _returnvalue (UserInterface|CreateWidget "/Game/UI/WB_InteractPrompt.WB_InteractPrompt_C"))
  (Variables|Default|SetInteractPrompt _returnvalue))

(event EventInteract
  (params (Player :type Character%20Object%20Reference))
  (CallFunction|RPCServerOpenMap))

(fn ConstructionScript)