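; BP_ResearchBase is an interactable research actor with a box trigger, intended to show a "Research" prompt to the player.
; On BeginPlay it creates a WB_InteractPrompt widget and stores it.
; The logic to show and remove that prompt for the player character is disconnected from the Box begin and end overlap events, so the prompt never appears.
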(event OnComponentBeginOverlap(Box)
  (params (OverlappedComponent :type Primitive%20Component%20Object%20Reference) (OtherActor :type Actor%20Object%20Reference) (OtherComp :type Primitive%20Component%20Object%20Reference) (OtherBodyIndex :type Integer) (bFromSweep :type Boolean) (SweepResult :type Hit%20Result%20Structure%20%28by%20ref%29)))

(event OnComponentEndOverlap(Box)
  (params (OverlappedComponent :type Primitive%20Component%20Object%20Reference) (OtherActor :type Actor%20Object%20Reference) (OtherComp :type Primitive%20Component%20Object%20Reference) (OtherBodyIndex :type Integer)))

(event EventBeginPlay
  (bind _returnvalue (UserInterface|CreateWidget "/Game/UI/WB_InteractPrompt.WB_InteractPrompt_C"))
  (Variables|Default|SetInteractPrompt _returnvalue))

(fn ConstructionScript)