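; Interactable door that toggles open and closed with a sound, either sliding or rotating depending on IsRotatingDoor, and shows a sign mesh set on BeginPlay.
; Open and lock requests pass through a server RPC to a second RPC that changes the state; a locked door ignores opening and closing.
; Timelines lerp the door's relative location or rotation and reverse to close.
; Power, light and room-tag getters are stubs returning empty defaults.
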(event Custom|OpenDoorDown
  (CallFunction|RPCServerOpenDoor))

(event Custom|SetLockStatus
  (CallFunction|RPCServerSetLockStatus))

(event Custom|RPC_SetLockStatus
  (if (not (Variables|Default|GetIsDoorLocked?))
    (Variables|Default|SetIsDoorLocked? true)
    (else
      (Variables|Default|SetIsDoorLocked? false))))

(event Custom|RPC_ServerSetLockStatus
  (CallFunction|RPCSetLockStatus))

(event Custom|RPC_OpenDoor
  (if (not (Variables|Default|GetIsDoorLocked?))
    (Audio|PlaySoundatLocation (Variables|Default|GetDoorSound) (Variables|/Script/Engine.SceneComponent|GetRelativeLocation (Variables|Default|GetDoor)) "0, 0, 0" 1.0 1.0 0.0 0 0 0 0)
    (if (not (Variables|Default|GetIsRotatingDoor?))
      (if (not (Variables|Default|GetIsDoorOpen?))
        (Variables|Default|SetIsDoorOpen? true)
        (bind _opentrack (Timeline|OpenDoorT Play)
          (:Update
            (Transformation|SetRelativeLocation (Variables|Default|GetDoor) (Math|Vector|Lerp(Vector) (Variables|Default|GetClosedPosition) (Variables|Default|GetOpenPosition) _opentrack) false false)))
        (else
          (Variables|Default|SetIsDoorOpen? false)
          (Timeline|OpenDoorT Reverse)))
      (elif (not (Variables|Default|GetIsDoorOpen?))
        (Variables|Default|SetIsDoorOpen? true)
        (bind _opentrack_2 (Timeline|Timeline Play)
          (:Update
            (Transformation|SetRelativeRotation (Variables|Default|GetDoor) (Math|Rotator|Lerp(Rotator) (Variables|Default|GetRotatingOpenPos) (Variables|Default|GetRotatingClosedPos) _opentrack_2) false false)))
        (else
          (Variables|Default|SetIsDoorOpen? false)
          (Timeline|Timeline Reverse))))))

(event Custom|RPC_ServerOpenDoor
  (CallFunction|RPCOpenDoor))

(event EventBeginPlay
  (Components|StaticMesh|SetStaticMesh (Variables|Default|GetSM_SignBorder_Fix_01) (Variables|Default|GetDoorSign)))

(fn ConstructionScript)

(fn GetCurrentPower
  (return 0))

(fn GetInteractRoomTag
  (return ""))

(fn GetLightStatus
  (return false))

(fn GetMaxPower
  (return 0))

(fn GetPowerOutage
  (return false))