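; BP_Signs is an interactable sign actor that applies a chosen static mesh at BeginPlay and shows a toggleable lock state.
; SetLockStatus passes through a server-named RPC event to RPC_SetLockStatus, where a FlipFlop alternates IsLocked and swaps the sign material between two variants.
; The toggle follows the FlipFlop's own internal state rather than reading IsLocked, starting with locked on the first call.
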(event Custom|SetLockStatus
  (CallFunction|RPCServerSetLockStatus))

(event Custom|RPC_SetLockStatus
  (bind _sign (Variables|Default|GetSign))
  (Utilities|FlowControl|FlipFlop
    (:A
      (Variables|Default|SetIsLocked? true)
      (Rendering|Material|SetMaterial _sign 0 "/Game/PolygonSciFiSpace/Materials/MAT_PolygonSciFiSpace_Signs_01_B.MAT_PolygonSciFiSpace_Signs_01_B"))
    (:B
      (Variables|Default|SetIsLocked? false)
      (Rendering|Material|SetMaterial _sign 0 "/Game/PolygonSciFiSpace/Materials/MAT_PolygonSciFiSpace_Signs_01_A.MAT_PolygonSciFiSpace_Signs_01_A"))))

(event Custom|RPC_ServerSetLockStatus
  (CallFunction|RPCSetLockStatus))

(event EventBeginPlay
  (Components|StaticMesh|SetStaticMesh (Variables|Default|GetSign) (Variables|Default|GetChosenSign)))

(fn ConstructionScript)