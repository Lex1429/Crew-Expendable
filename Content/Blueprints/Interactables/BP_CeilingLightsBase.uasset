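; BP_CeilingLightsBase is a base ceiling light that can be toggled on and off.
; ToggleLight routes through a server RPC to RPC_ToggleLight, which flips IsLightOn and sets the tile material's LightStrength parameter.
; An active PowerOutage forces the light off.
; GetLightStatus reports the state, while the power and room-tag getters return placeholder values and an older FlipFlop toggle is left unconnected.
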(event Custom|ToggleLight
  (CallFunction|RPCServerToggleLight))

(event Custom|RPC_ToggleLight
  (if (Variables|Default|GetPowerOutage?)
    (Rendering|Material|SetScalarParameterValueonMaterials (Variables|Default|GetCealingTile) "LightStrength" 0.0)
    (Variables|Default|SetIsLightOn? false)
    (elif (Variables|Default|GetIsLightOn?)
      (Rendering|Material|SetScalarParameterValueonMaterials (Variables|Default|GetCealingTile) "LightStrength" 0.0)
      (Variables|Default|SetIsLightOn? false)
      (else
        (Rendering|Material|SetScalarParameterValueonMaterials (Variables|Default|GetCealingTile) "LightStrength" 1.0)
        (Variables|Default|SetIsLightOn? true)))))

(event Custom|RPC_ServerToggleLight
  (CallFunction|RPCToggleLight))

(fn ConstructionScript)

(fn GetCurrentPower
  (return 0))

(fn GetInteractRoomTag
  (return ""))

(fn GetLightStatus
  (return (Variables|Default|GetIsLightOn?)))

(fn GetMaxPower
  (return 0))

(fn GetPowerOutage
  (return false))