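; BP_DoorSwitch is an interactable switch that opens its matching BP_SMDoor1 door.
; A box overlap by player 0's character shows or hides an interact prompt widget created at BeginPlay.
; Interact chains through a server-named RPC event to a second RPC event, which searches all doors and calls OpenDoorDown on the first whose DoorValue equals the switch's ButtonValue.
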(event OnComponentBeginOverlap(Box)
  (params (OverlappedComponent :type Primitive%20Component%20Object%20Reference) (OtherActor :type Actor%20Object%20Reference) (OtherComp :type Primitive%20Component%20Object%20Reference) (OtherBodyIndex :type Integer) (bFromSweep :type Boolean) (SweepResult :type Hit%20Result%20Structure%20%28by%20ref%29))
  (if (== OtherActor (Game|GetPlayerCharacter 0))
    (UserInterface|Viewport|AddtoViewport (Variables|Default|GetInteractPrompt) 0)))

(event OnComponentEndOverlap(Box)
  (params (OverlappedComponent :type Primitive%20Component%20Object%20Reference) (OtherActor :type Actor%20Object%20Reference) (OtherComp :type Primitive%20Component%20Object%20Reference) (OtherBodyIndex :type Integer))
  (if (== (Game|GetPlayerCharacter 0) OtherActor)
    (Widget|RemovefromParent (Variables|Default|GetInteractPrompt))))

(event Custom|RPC_DoorSwitchInteract
  (bind _outactors (Actor|GetAllActorsOfClass "/Game/Blueprints/Interactables/BP_SMDoor1.BP_SMDoor1_C"))
  (bind _array_element (Utilities|Array|ForEachLoopwithBreak _outactors :!label _label)
    (:LoopBody
      (if (== (Variables|/Game/Blueprints/Interactables/BP_SMDoor1.BP_SMDoor1_C|GetDoorValue _array_element) (Variables|Default|GetButtonValue))
        (Default|OpenDoorDown _array_element)
        (goto _label Break)))))

(event Custom|RPC_ServerDoorSwitchInteract
  (CallFunction|RPCDoorSwitchInteract))

(event EventBeginPlay
  (bind _returnvalue (UserInterface|CreateWidget "/Game/UI/WB_InteractPrompt.WB_InteractPrompt_C"))
  (Variables|Default|SetInteractPrompt _returnvalue))

(event EventInteract
  (params (Player :type Character%20Object%20Reference))
  (CallFunction|RPCServerDoorSwitchInteract))

(fn ConstructionScript)