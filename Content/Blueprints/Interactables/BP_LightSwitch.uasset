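; Interactable light switch that toggles every ceiling light belonging to its assigned room.
; Its box overlap shows or hides an interact prompt for the player character, labelled with the room's lights name.
; Interact goes through a server RPC into a second RPC, which finds all BP_CeilingLightsBase actors whose tag matches the room's and toggles them.
; Light status and power outage getters are stubs returning false.
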(event OnComponentBeginOverlap(Box)
  (params (OverlappedComponent :type Primitive%20Component%20Object%20Reference) (OtherActor :type Actor%20Object%20Reference) (OtherComp :type Primitive%20Component%20Object%20Reference) (OtherBodyIndex :type Integer) (bFromSweep :type Boolean) (SweepResult :type Hit%20Result%20Structure%20%28by%20ref%29))
  (bind _interactprompt (Variables|Default|GetInteractPrompt))
  (if (== OtherActor (Game|GetPlayerCharacter 0))
    (UserInterface|Viewport|AddtoViewport _interactprompt 0)
    (Rendering|Components|TextRender|SetText (Variables|/Game/UI/WB_InteractPrompt.WB_InteractPrompt_C|GetStatusText _interactprompt) (Utilities|Text|ToText(Name) (.LightsName (CallFunction|GetRoomDetails (Variables|Default|GetRoom%20Tag%20In)))))))

(event OnComponentEndOverlap(Box)
  (params (OverlappedComponent :type Primitive%20Component%20Object%20Reference) (OtherActor :type Actor%20Object%20Reference) (OtherComp :type Primitive%20Component%20Object%20Reference) (OtherBodyIndex :type Integer))
  (if (== (Game|GetPlayerCharacter 0) OtherActor)
    (Widget|RemovefromParent (Variables|Default|GetInteractPrompt))))

(event Custom|RPC_LightSwitchInteract
  (bind _outactors (Actor|GetAllActorsOfClass "/Game/Blueprints/Interactables/BP_CeilingLightsBase.BP_CeilingLightsBase_C"))
  (bind _array_element (Utilities|Array|ForEachLoopwithBreak _outactors)
    (:LoopBody
      (if (== (Variables|/Game/Blueprints/Interactables/BP_CeilingLightsBase.BP_CeilingLightsBase_C|GetLightsTag _array_element) (.RoomTag (CallFunction|GetRoomDetails (Variables|Default|GetRoom%20Tag%20In))))
        (Default|ToggleLight _array_element)))))

(event Custom|RPC_ServerLightSwitchInteract
  (CallFunction|RPCLightSwitchInteract))

(event EventBeginPlay
  (bind _returnvalue (UserInterface|CreateWidget "/Game/UI/WB_InteractPrompt.WB_InteractPrompt_C"))
  (Variables|Default|SetInteractPrompt _returnvalue))

(event EventInteract
  (params (Player :type Character%20Object%20Reference))
  (CallFunction|RPCServerLightSwitchInteract))

(fn ConstructionScript)

(fn GetLightStatus
  (return false))

(fn GetPowerOutage
  (return false))