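; BP_Drone_Flying_01 is a drone actor that flies along a spline path placed in the level.
; On BeginPlay it finds a BP_SPline_DRone actor by class and starts a timeline whose play rate is the inverse of TimeToCOmplete.
; Each timeline update maps the track value to a distance along the spline and sets the drone's transform there, using world-space location but local-space rotation.
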(event Custom|Move
  (bind _spline_drone (Variables|Default|GetSpline_Drone))
  (bind _spline (Variables|/Game/PolygonSciFiWorlds/FX/Spline/BP_SPline_DRone.BP_SPline_DRone_C|GetSpline _spline_drone))
  (Components|Timeline|SetPlayRate (Variables|Default|GetObject%20movement) (/ 1.0 (Variables|Default|GetTime%20to%20COmplete)))
  (bind _newtrack_0 (Timeline|Object%20movement Play)
    (:Update
      (Transformation|SetActorTransform (Math|Transform|MakeTransform (Spline|GetLocationatDistanceAlongSpline _spline (Math|Float|Lerp 0.0 (Spline|GetSplineLength (Variables|/Game/PolygonSciFiWorlds/FX/Spline/BP_SPline_DRone.BP_SPline_DRone_C|GetSpline (Variables|Default|GetSpline_Drone))) _newtrack_0) "World") (Spline|GetRotationatDistanceAlongSpline _spline (Math|Float|Lerp 0.0 (Spline|GetSplineLength (Variables|/Game/PolygonSciFiWorlds/FX/Spline/BP_SPline_DRone.BP_SPline_DRone_C|GetSpline (Variables|Default|GetSpline_Drone))) _newtrack_0) "Local") "1.000000,1.000000,1.000000")))))

(event EventBeginPlay
  (bind _returnvalue (Actor|GetActorOfClass "/Game/PolygonSciFiWorlds/FX/Spline/BP_SPline_DRone.BP_SPline_DRone_C"))
  (Variables|Default|SetSpline_Drone _returnvalue)
  (CallFunction|Move))

(fn ConstructionScript)