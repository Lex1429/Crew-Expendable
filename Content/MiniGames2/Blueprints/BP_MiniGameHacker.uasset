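; Hacking minigame actor: the player moves a selector across three symbol columns, scrolls them to match a random target, and confirms until all three are solved.
; A looping timer polls input while a dynamic screen material renders columns, selector and results, with a timeline animating scrolls.
; A wrong confirm resets progress and reshuffles symbols on Tick.
; Activation blends to the game camera and temporarily overrides TAA frame weight for sharper text.
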(event OnComponentBeginOverlap(InteractionBoundBox)
  (params (OverlappedComponent :type Primitive%20Component%20Object%20Reference) (OtherActor :type Actor%20Object%20Reference) (OtherComp :type Primitive%20Component%20Object%20Reference) (OtherBodyIndex :type Integer) (bFromSweep :type Boolean) (SweepResult :type Hit%20Result%20Structure%20%28by%20ref%29))
  ;[1 1 1] Player overlapping
  (CallFunction|CheckBeginOverlap OtherActor))

(event OnComponentEndOverlap(InteractionBoundBox)
  (params (OverlappedComponent :type Primitive%20Component%20Object%20Reference) (OtherActor :type Actor%20Object%20Reference) (OtherComp :type Primitive%20Component%20Object%20Reference) (OtherBodyIndex :type Integer))
  ;[1 1 1] Player overlapping
  (CallFunction|CheckEndOverlap OtherActor))

(event Custom|CheckContorls
  (bind _rightaxis (Variables|Default|GetRightAxis))
  (bind _forwardaxis (Variables|Default|GetForwardAxis))
  ;[1 1 1] Controls
  (if (Variables|Default|GetInputEnable)
    (if (Variables|Default|GetIsMiniGameActivated)
      (Utilities|FlowControl|Sequence
        (:then_0
          (if (!= _rightaxis 0.0)
            (if (Variables|Default|GetRightAxisEnable)
              (Variables|Default|SetRightAxisEnable false)
              (bind _newindex (CallFunction|GetSolverIndexX (Variables|Default|GetSelectorIndex) (Math|Float|Truncate (Math|Float|Sign(Float) _rightaxis))))
              (bind _output_get (Variables|Default|SetSelectorIndex _newindex))
              (Rendering|Material|SetScalarParameterValue (Variables|Default|GetDMI) "Selector_X" (Math|Conversions|ToFloat(Integer) _output_get) :!class /Script/Engine.MaterialInstanceDynamic))
            (else
              (Variables|Default|SetRightAxisEnable true))))
        (:then_1
          (if (!= _forwardaxis 0.0)
            (Variables|Default|SetFromY (- (* (Utilities|Array|Get(acopy) (Variables|Default|GetColumns_IndexY) (Variables|Default|GetSelectorIndex)) 0.25) 0.67))
            (bind _output_get_2 (Variables|Default|SetResult (Math|Integer|Clamp(Integer) (+ (Utilities|Array|Get(acopy) (Variables|Default|GetColumns_IndexY) (Variables|Default|GetSelectorIndex)) (Math|Float|Truncate (Math|Float|Sign(Float) _forwardaxis))) 0 7)))
            (if (not (== _output_get_2 (Utilities|Array|Get(acopy) (Variables|Default|GetColumns_IndexY) (Variables|Default|GetSelectorIndex))))
              (Variables|Default|SetToY (- (* (Variables|Default|GetResult) 0.25) 0.67))
              (Variables|Default|SetInputEnable false)
              (bind _newtrack_0 (Timeline|Timeline_0 PlayFromStart)
                (:Update
                  (Rendering|Material|SetScalarParameterValue (Variables|Default|GetDMI) (Utilities|String|StringToName (Utilities|String|Append "Col" (Utilities|String|ToString(Integer) (+ (Variables|Default|GetSelectorIndex) 1)) "_Y")) (Math|Float|Lerp (Variables|Default|GetFromY) (Variables|Default|GetToY) _newtrack_0) :!class /Script/Engine.MaterialInstanceDynamic))
                (:Finished
                  (Variables|Default|SetInputEnable true)
                  (|SetBy-RefVar (Utilities|Array|Get(acopy) (Variables|Default|GetColumns_IndexY) (Variables|Default|GetSelectorIndex)) (Variables|Default|GetResult)))))))))))

(event Custom|SetupSolver
  (bind _dmi (Variables|Default|GetDMI))
  ;[1 1 1] Setup randomly Solver
  (bind _output_get (Variables|Default|SetSolverData (Utilities|Struct|MakeF_MG_HackerSolver (CallFunction|GetSolverRandomX) (Math|Random|RandomIntegerinRange 0 7))))
  (Rendering|Material|SetScalarParameterValue _dmi "Solver_X" (Math|Conversions|ToFloat(Integer) (.Index_X (Utilities|Struct|BreakF_MG_HackerSolver (Utilities|Array|Get(acopy) (Variables|Default|GetSymbolsData) (.Index_X (Utilities|Struct|BreakF_MG_HackerSolver _output_get)))))) :!class /Script/Engine.MaterialInstanceDynamic)
  (Rendering|Material|SetScalarParameterValue _dmi "Solver_Y" (Math|Conversions|ToFloat(Integer) (.Index_Y (Utilities|Struct|BreakF_MG_HackerSolver _output_get))) :!class /Script/Engine.MaterialInstanceDynamic)
  (Development|PrintString (Utilities|String|Append "Solver Col (X): " (Utilities|String|ToString(Integer) (.Index_X (Utilities|Struct|BreakF_MG_HackerSolver _output_get))) " Row (Y): " (Utilities|String|ToString(Integer) (.Index_Y (Utilities|Struct|BreakF_MG_HackerSolver _output_get)))) true true "(R=0.000000,G=1.000000,B=0.000000,A=1.000000)" 1e+01)
  (Rendering|Material|SetScalarParameterValue (Variables|Default|GetDMI) "Selector_X" (Math|Conversions|ToFloat(Integer) (Variables|Default|GetSelectorIndex)) :!class /Script/Engine.MaterialInstanceDynamic))

(event Custom|InitGame
  ;[1 1 1] ReInit game
  ;;[0 0.1488 1] Set TAA Current Fram Weight for increasing text rendering quality
  (bind _returnvalue (Development|GetConsoleVariableFloatValue "r.TemporalAACurrentFrameWeight"))
  (Variables|Default|SetGameTAACurrFrameWeight _returnvalue)
  (Development|ExecuteConsoleCommand (Game|GetPlayerController 0) "r.TemporalAACurrentFrameWeight 0.15" 0)
  (Utilities|Array|Clear (Variables|Default|GetSymbolsData))
  (Variables|Default|SetRightAxisEnable true)
  (Variables|Default|SetReinit false)
  (Rendering|Material|SetScalarParameterValue (Variables|Default|GetDMI) "ShowError" 0.0 :!class /Script/Engine.MaterialInstanceDynamic)
  (Rendering|Material|SetScalarParameterValue (Variables|Default|GetDMI) "ShowHacked" 0.0 :!class /Script/Engine.MaterialInstanceDynamic)
  (Variables|Default|SetSelectorIndex 1)
  (Utilities|Array|Clear (Variables|Default|GetColumns_IndexY))
  (for _index (range 0 10)
    (CallFunction|ManualSwap (Math|Random|RandomIntegerinRange 0 7) (Math|Random|RandomIntegerinRange 0 7)))
  (CallFunction|SetupColumns)
  (CallFunction|SetupSolver)
  (Variables|Default|SetInputEnable true))

(event Custom|SetupColumns
  (bind _symbolsdata (Variables|Default|GetSymbolsData))
  (bind _columns_indexy (Variables|Default|GetColumns_IndexY))
  (bind _symbolsdata_2 (Variables|Default|GetSymbolsData))
  (bind _dmi (Variables|Default|GetDMI))
  (bind _symbolsdata_3 (Variables|Default|GetSymbolsData))
  (bind _output (Utilities|Array|Get(acopy) _symbolsdata_3 2))
  (bind _output_2 (Utilities|Array|Get(acopy) _symbolsdata_3))
  (bind _output_3 (Utilities|Array|Get(acopy) _symbolsdata_3 1))
  (bind _index_y (Utilities|Struct|BreakF_MG_HackerSolver _output))
  (bind _index_y_2 (Utilities|Struct|BreakF_MG_HackerSolver _output_2))
  (bind _index_y_3 (Utilities|Struct|BreakF_MG_HackerSolver _output_3))
  ;[1 1 1] Setup randomly columns
  (Utilities|Array|Add _symbolsdata_2 (Utilities|Struct|MakeF_MG_HackerSolver (Utilities|Array|Get(acopy) (Variables|Default|GetSymbolIndices)) (Math|Random|RandomIntegerinRange 0 7)))
  (Utilities|Array|Add _symbolsdata_2 (Utilities|Struct|MakeF_MG_HackerSolver (Utilities|Array|Get(acopy) (Variables|Default|GetSymbolIndices) 1) (Math|Random|RandomIntegerinRange 0 7)))
  (Utilities|Array|Add _symbolsdata_2 (Utilities|Struct|MakeF_MG_HackerSolver (Utilities|Array|Get(acopy) (Variables|Default|GetSymbolIndices) 2) (Math|Random|RandomIntegerinRange 0 7)))
  (Rendering|Material|SetScalarParameterValue _dmi "Col1_X" (Math|Conversions|ToFloat(Integer) (.Index_X (Utilities|Struct|BreakF_MG_HackerSolver (Utilities|Array|Get(acopy) _symbolsdata)))) :!class /Script/Engine.MaterialInstanceDynamic)
  (Rendering|Material|SetScalarParameterValue _dmi "Col2_X" (Math|Conversions|ToFloat(Integer) (.Index_X (Utilities|Struct|BreakF_MG_HackerSolver (Utilities|Array|Get(acopy) _symbolsdata 1)))) :!class /Script/Engine.MaterialInstanceDynamic)
  (Rendering|Material|SetScalarParameterValue _dmi "Col3_X" (Math|Conversions|ToFloat(Integer) (.Index_X (Utilities|Struct|BreakF_MG_HackerSolver (Utilities|Array|Get(acopy) _symbolsdata 2)))) :!class /Script/Engine.MaterialInstanceDynamic)
  (Utilities|Array|Add _columns_indexy _index_y_2)
  (Rendering|Material|SetScalarParameterValue (Variables|Default|GetDMI) "Col1_Y" (- (* _index_y_2 0.25) 0.67) :!class /Script/Engine.MaterialInstanceDynamic)
  (Utilities|Array|Add _columns_indexy _index_y_3)
  (Rendering|Material|SetScalarParameterValue (Variables|Default|GetDMI) "Col2_Y" (- (* _index_y_3 0.25) 0.67) :!class /Script/Engine.MaterialInstanceDynamic)
  (Utilities|Array|Add _columns_indexy _index_y)
  (Rendering|Material|SetScalarParameterValue (Variables|Default|GetDMI) "Col3_Y" (- (* _index_y 0.25) 0.67) :!class /Script/Engine.MaterialInstanceDynamic))

(event Custom|ManualSwap
  (params (Index1 :type Integer) (Index2 :type Integer))
  (bind _symbolindices (Variables|Default|GetSymbolIndices))
  ;[1 0.07657 0] For Nativization compatibility
  (Variables|Default|SetInd1 Index1)
  (Variables|Default|SetInd2 Index2)
  (Variables|Default|SetVal1 (Utilities|Array|Get(acopy) _symbolindices (Variables|Default|GetInd1)))
  (Variables|Default|SetVal2 (Utilities|Array|Get(acopy) _symbolindices (Variables|Default|GetInd2)))
  (Utilities|Array|SetArrayElem _symbolindices (Variables|Default|GetInd1) (Variables|Default|GetVal2))
  (Utilities|Array|SetArrayElem _symbolindices (Variables|Default|GetInd2) (Variables|Default|GetVal1)))

(event EventBeginPlay
  ;[1 1 1] Init
  (|CallParentFunction)
  (Variables|Default|SetIsMiniGameActivated false)
  (Variables|Default|SetInputEnable false)
  (bind _returnvalue (Rendering|Material|CreateDynamicMaterialInstance "/Game/MiniGames2/Materials/MI_MiniGamesHacker_Inst.MI_MiniGamesHacker_Inst" "None" :!class /Script/Engine.KismetMaterialLibrary))
  (Variables|Default|SetDMI _returnvalue)
  (bind _returnvalue_2 (Utilities|Time|SetTimerbyFunctionName 0 "CheckContorls" 0.05 true))
  (Variables|Default|SetTimeHandle _returnvalue_2))

(event Collision|EventActorBeginOverlap
  (params (OtherActor :type Actor%20Object%20Reference))
  (|CallParentFunction OtherActor) ; This node is disabled and will not be called.\nDrag off pins to build functionality.
)

(event EventTick
  (params (DeltaSeconds :type Float%20%28single-precision%29))
  (bind _dmi (Variables|Default|GetDMI))
  ;[1 1 1] ReInit activation / cycling
  (|CallParentFunction DeltaSeconds)
  (if (Variables|Default|GetIsMiniGameActivated)
    (if (Variables|Default|GetReinit)
      (if (>= (Variables|Default|GetCounter) 35)
        (Variables|Default|SetReinit false)
        (bind _output_get (Variables|Default|SetSelectorIndex 1))
        (Rendering|Material|SetScalarParameterValue (Variables|Default|GetDMI) "Selector_X" (Math|Conversions|ToFloat(Integer) _output_get) :!class /Script/Engine.MaterialInstanceDynamic)
        (Utilities|Array|Clear (Variables|Default|GetSymbolsData))
        (Utilities|Array|Clear (Variables|Default|GetColumns_IndexY))
        (CallFunction|SetupColumns)
        (CallFunction|SetupSolver)
        (Rendering|Material|SetScalarParameterValue (Variables|Default|GetDMI) "ShowError" 0.0 :!class /Script/Engine.MaterialInstanceDynamic)
        (Variables|Default|SetInputEnable true)
        (elif (>= (- (Utilities|Time|GetGameTimeinSeconds) (Variables|Default|GetStartTime)) 0.035)
          (CallFunction|ManualSwap (Math|Random|RandomIntegerinRange 0 7) (Math|Random|RandomIntegerinRange 0 7))
          (Variables|Default|SetStartTime (Utilities|Time|GetGameTimeinSeconds))
          (Math|Integer|IncrementInt (Variables|Default|GetCounter)
            (:%20%20
              (Rendering|Material|SetScalarParameterValue _dmi "Col1_X" (Math|Conversions|ToFloat(Integer) (Math|Random|RandomIntegerinRange 0 7)) :!class /Script/Engine.MaterialInstanceDynamic)
              (Rendering|Material|SetScalarParameterValue _dmi "Col2_X" (Math|Conversions|ToFloat(Integer) (Math|Random|RandomIntegerinRange 0 7)) :!class /Script/Engine.MaterialInstanceDynamic)
              (Rendering|Material|SetScalarParameterValue _dmi "Col3_X" (Math|Conversions|ToFloat(Integer) (Math|Random|RandomIntegerinRange 0 7)) :!class /Script/Engine.MaterialInstanceDynamic)
              (Rendering|Material|SetScalarParameterValue _dmi "Col1_Y" (Math|Conversions|ToFloat(Integer) (Math|Random|RandomIntegerinRange 0 7)) :!class /Script/Engine.MaterialInstanceDynamic)
              (Rendering|Material|SetScalarParameterValue _dmi "Col2_Y" (Math|Conversions|ToFloat(Integer) (Math|Random|RandomIntegerinRange 0 7)) :!class /Script/Engine.MaterialInstanceDynamic)
              (Rendering|Material|SetScalarParameterValue _dmi "Col3_Y" (Math|Conversions|ToFloat(Integer) (Math|Random|RandomIntegerinRange 0 7)) :!class /Script/Engine.MaterialInstanceDynamic))))))))

(event EventForceAction
  (bind _errorsound (Variables|Default|GetErrorSound))
  (bind _solverdata (Variables|Default|GetSolverData))
  (bind _dmi (Variables|Default|GetDMI))
  (bind (_index_x _index_y) (Utilities|Struct|BreakF_MG_HackerSolver _solverdata))
  ;[1 1 1] Action button
  (if (Variables|Default|GetPlayerOverlapped)
    (if (Variables|Default|GetIsMiniGameActivated)
      (if (Variables|Default|GetInputEnable)
        (Variables|Default|SetInputEnable false)
        (if (and (== _index_x (Variables|Default|GetSelectorIndex)) (== _index_y (Utilities|Array|Get(acopy) (Variables|Default|GetColumns_IndexY) (Variables|Default|GetSelectorIndex))))
          (|SetBy-RefVar (Utilities|Array|Get(acopy) (Variables|Default|GetColumns_IndexY) (Variables|Default|GetSelectorIndex)) -1)
          (Rendering|Material|SetScalarParameterValue (Variables|Default|GetDMI) (Utilities|String|StringToName (Utilities|String|Append "Col" (Utilities|String|ToString(Integer) (+ (Variables|Default|GetSelectorIndex) 1)) "_Solved")) 1.0 :!class /Script/Engine.MaterialInstanceDynamic)
          (bind _result (Math|Integer|IncrementInt (Variables|Default|GetSolved))
            (:%20%20
              (if (== _result 3)
                ;;[1 1 1] Success
                (Variables|Default|SetMiniGameEnabled false)
                (Variables|Default|SetIsMiniGameActivated false)
                (Variables|Default|SetInputEnable false)
                (Rendering|Material|SetScalarParameterValue (Variables|Default|GetDMI) "ShowHacked" 1.0 :!class /Script/Engine.MaterialInstanceDynamic)
                (Utilities|FlowControl|Delay (Variables|Default|GetDelayTimeWhenComplete))
                (CallFunction|SetOfflineMaterial)
                (Default|CallOnMiniGameSuccess)
                (Development|ExecuteConsoleCommand (Game|GetPlayerController 0) (Utilities|String|Append "r.TemporalAACurrentFrameWeight " (Utilities|String|ToString(Float) (Variables|Default|GetGameTAACurrFrameWeight))) 0)
                (CallFunction|BlendCamerafromGametoPlayer (Variables|Default|GetOverlappedActor))
                (else
                  (Variables|Default|SetSelectorIndex (CallFunction|GetSolverRandomX))
                  (CallFunction|SetupSolver)
                  (Variables|Default|SetInputEnable true)))))
          (else
            ;;[1 1 1] Error
            (Variables|Default|SetCounter 0)
            (Rendering|Material|SetScalarParameterValue _dmi "Col1_Solved" 0.0 :!class /Script/Engine.MaterialInstanceDynamic)
            (Rendering|Material|SetScalarParameterValue _dmi "Col2_Solved" 0.0 :!class /Script/Engine.MaterialInstanceDynamic)
            (Rendering|Material|SetScalarParameterValue _dmi "Col3_Solved" 0.0 :!class /Script/Engine.MaterialInstanceDynamic)
            (Rendering|Material|SetScalarParameterValue _dmi "ShowError" 1.0 :!class /Script/Engine.MaterialInstanceDynamic)
            (Variables|Default|SetSolved 0)
            (Variables|Default|SetReinit true)
            (Utilities|IsValid _errorsound
              (:Is%20Valid
                (Audio|PlaySoundatLocation _errorsound (Transformation|GetActorLocation self) "0, 0, 0" 1.0 1.0 0.0 0 0 0))))))
      (else
        (CallFunction|InitGame)
        (Rendering|Material|SetMaterial (Variables|Default|GetMiniGameScreen) 0 (Variables|Default|GetDMI))
        (CallFunction|BlendCamerafromPlayertoGame self (Variables|Default|GetOverlappedActor))
        (Variables|Default|SetIsMiniGameActivated true)
        (Variables|Default|SetInputEnable true)))))

(event EventForceExit
  ;[1 1 1] Cancel
  (if (and (Variables|Default|GetMiniGameEnabled) (Variables|Default|GetIsMiniGameActivated))
    (Variables|Default|SetIsMiniGameActivated false)
    (Variables|Default|SetInputEnable false)
    ;;[0 0.1488 1] Restore TAA Current Weight Frame value
    (Development|ExecuteConsoleCommand (Game|GetPlayerController 0) (Utilities|String|Append "r.TemporalAACurrentFrameWeight " (Utilities|String|ToString(Float) (Variables|Default|GetGameTAACurrFrameWeight))) 0)
    (Default|CallOnMiniGameCanceled)
    (CallFunction|BlendCamerafromGametoPlayer (Variables|Default|GetOverlappedActor))))

(fn ConstructionScript
  (|CallParentFunction))

(fn GetSolverIndexX
  (params (Index :type Integer) (Sign :type Integer))
  ;[1 1 1] Return current Solver column Index
  (bind _output_get (LocalVariables|SetOutIndex Index))
  (if (>= (Utilities|Array|Get(acopy) (Variables|Default|GetColumns_IndexY) (Math|Integer|Clamp(Integer) (+ _output_get Sign) 0 2)) 0)
    (LocalVariables|SetOutIndex (Math|Integer|Clamp(Integer) (+ _output_get Sign) 0 2))
    (elif (>= (Utilities|Array|Get(acopy) (Variables|Default|GetColumns_IndexY) (Math|Integer|Clamp(Integer) (+ (Math|Integer|Clamp(Integer) (+ _output_get Sign) 0 2) Sign) 0 2)) 0)
      (LocalVariables|SetOutIndex (+ (Math|Integer|Clamp(Integer) (+ _output_get Sign) 0 2) Sign))))
  (return (LocalVariables|GetOutIndex)))

(fn GetSolverRandomX
  (bind _columns_indexy (Variables|Default|GetColumns_IndexY))
  (bind _tempindex (LocalVariables|GetTempIndex))
  (bind _tempindex_2 (LocalVariables|GetTempIndex))
  ;[1 1 1] Ger random Solver index
  (Utilities|FlowControl|Sequence
    (:then_0
      (if (>= (Utilities|Array|Get(acopy) _columns_indexy) 0)
        (Utilities|Array|Add _tempindex 0)))
    (:then_1
      (if (>= (Utilities|Array|Get(acopy) _columns_indexy 1) 0)
        (Utilities|Array|Add _tempindex 1)))
    (:then_2
      (if (>= (Utilities|Array|Get(acopy) _columns_indexy 2) 0)
        (Utilities|Array|Add _tempindex 2)))
    (:then_3
      (return (Utilities|Array|Get(acopy) _tempindex_2 (Math|Random|RandomIntegerinRange 0 (- (Utilities|Array|Length _tempindex_2) 1)))))))