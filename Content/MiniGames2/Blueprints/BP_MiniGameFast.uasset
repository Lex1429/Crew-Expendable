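; Timing minigame on an in-world screen: the player stops a sweeping marker inside each bar's randomly placed target segment.
; Two to four bars, drawn through a dynamic material, run in sequence while Tick bounces the marker at per-bar speeds.
; A miss flashes the bar, then re-randomizes it and steps back one bar.
; Clearing all bars fires success, returns the camera and increments the GameState research data message.
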(event OnComponentBeginOverlap(InteractionBoundBox)
  (params (OverlappedComponent :type Primitive%20Component%20Object%20Reference) (OtherActor :type Actor%20Object%20Reference) (OtherComp :type Primitive%20Component%20Object%20Reference) (OtherBodyIndex :type Integer) (bFromSweep :type Boolean) (SweepResult :type Hit%20Result%20Structure%20%28by%20ref%29))
  ;[1 1 1] Player overlapping
  (CallFunction|CheckBeginOverlap OtherActor))

(event OnComponentEndOverlap(InteractionBoundBox)
  (params (OverlappedComponent :type Primitive%20Component%20Object%20Reference) (OtherActor :type Actor%20Object%20Reference) (OtherComp :type Primitive%20Component%20Object%20Reference) (OtherBodyIndex :type Integer))
  ;[1 1 1] Player overlapping
  (CallFunction|CheckEndOverlap OtherActor))

(event Custom|SetTarget
  (params (BarNumber :type Integer) (UseHalf :type Boolean))
  (bind _returnvalue (+ BarNumber 1))
  (bind _dmi (Variables|Default|GetDMI))
  (bind _returnvalue_2 (Utilities|String|ToString(Integer) _returnvalue))
  ;[1 1 1] Set target based on target params
  (bind _output_get (Variables|Default|SetTargetPos (Math|Random|RandomIntegerinRange 0 7)))
  (switch int BarNumber
    (:0
      (Variables|Default|SetBar1_TargetIndex (Variables|Default|GetTargetPos))
      (Variables|Default|SetBar1_Half UseHalf))
    (:1
      (Variables|Default|SetBar2_TargetIndex (Variables|Default|GetTargetPos))
      (Variables|Default|SetBar2_Half UseHalf))
    (:2
      (Variables|Default|SetBar3_TargetIndex (Variables|Default|GetTargetPos))
      (Variables|Default|SetBar3_Half UseHalf))
    (:3
      (Variables|Default|SetBar4_TargetIndex (Variables|Default|GetTargetPos))
      (Variables|Default|SetBar4_Half UseHalf)))
  (Rendering|Material|SetScalarParameterValue _dmi (Utilities|String|StringToName (Utilities|String|Append "Bar" _returnvalue_2 "_" "Target" (Utilities|String|ToString(Integer) (+ _output_get 1)))) 1.0 :!class /Script/Engine.MaterialInstanceDynamic)
  (Rendering|Material|SetScalarParameterValue _dmi (Utilities|String|StringToName (Utilities|String|Append "Bar" _returnvalue_2 "_" "Usehalf")) (Math|Float|SelectFloat 1.0 0.0 UseHalf) :!class /Script/Engine.MaterialInstanceDynamic))

(event Custom|ResetBar
  (params (BarNumber :type Integer) (State :type Float%20%28double-precision%29) (UseHalf :type Float%20%28double-precision%29) (Color :type Linear%20Color%20Structure))
  (bind _returnvalue (+ BarNumber 1))
  (bind _dmi (Variables|Default|GetDMI))
  (bind _returnvalue_2 (Utilities|String|ToString(Integer) _returnvalue))
  ;[1 1 1] Reset bar to default state
  (for _index (range 1 8)
    (Rendering|Material|SetScalarParameterValue _dmi (Utilities|String|StringToName (Utilities|String|Append "Bar" _returnvalue_2 "_" "Target" (Utilities|String|ToString(Integer) _index))) State :!class /Script/Engine.MaterialInstanceDynamic)
    (Rendering|Material|SetScalarParameterValue _dmi (Utilities|String|StringToName (Utilities|String|Append "Bar" _returnvalue_2 "_" "Usehalf")) UseHalf :!class /Script/Engine.MaterialInstanceDynamic)
    (Rendering|Material|SetVectorParameterValue _dmi (Utilities|String|StringToName (Utilities|String|Append "Bar" _returnvalue_2 "_" "StatusColor")) Color :!class /Script/Engine.MaterialInstanceDynamic)))

(event Custom|InitGame
  (bind _dmi (Variables|Default|GetDMI))
  (bind _dmi_2 (Variables|Default|GetDMI))
  (bind _barcolornormal (Variables|Fast|GetBarColorNormal))
  ;[1 1 1] ReInit game
  (CallFunction|ResetBar 0 0.0 0.0 _barcolornormal)
  (CallFunction|ResetBar 1 0.0 0.0 _barcolornormal)
  (CallFunction|ResetBar 2 0.0 0.0 _barcolornormal)
  (CallFunction|ResetBar 3 0.0 0.0 _barcolornormal)
  (switch Utilities|FlowControl|Switch|SwitchonE_MG_FastCount (Variables|Fast|GetBarsCount)
    (:NewEnumerator0
      (Rendering|Material|SetScalarParameterValue _dmi_2 "Bar3_Vis" 0.0 :!class /Script/Engine.MaterialInstanceDynamic)
      (Rendering|Material|SetScalarParameterValue _dmi_2 "Bar4_Vis" 0.0 :!class /Script/Engine.MaterialInstanceDynamic)
      (Rendering|Material|SetScalarParameterValue _dmi_2 "Bar1_OY" 0.3 :!class /Script/Engine.MaterialInstanceDynamic)
      (Rendering|Material|SetScalarParameterValue _dmi_2 "Bar2_OY" 0.2 :!class /Script/Engine.MaterialInstanceDynamic))
    (:NewEnumerator1
      (Rendering|Material|SetScalarParameterValue _dmi_2 "Bar3_Vis" 1.0 :!class /Script/Engine.MaterialInstanceDynamic)
      (Rendering|Material|SetScalarParameterValue _dmi_2 "Bar4_Vis" 0.0 :!class /Script/Engine.MaterialInstanceDynamic)
      (Rendering|Material|SetScalarParameterValue _dmi_2 "Bar1_OY" 0.35 :!class /Script/Engine.MaterialInstanceDynamic)
      (Rendering|Material|SetScalarParameterValue _dmi_2 "Bar2_OY" 0.25 :!class /Script/Engine.MaterialInstanceDynamic)
      (Rendering|Material|SetScalarParameterValue _dmi_2 "Bar3_OY" 0.15 :!class /Script/Engine.MaterialInstanceDynamic))
    (:NewEnumerator2
      (Rendering|Material|SetScalarParameterValue _dmi_2 "Bar3_Vis" 1.0 :!class /Script/Engine.MaterialInstanceDynamic)
      (Rendering|Material|SetScalarParameterValue _dmi_2 "Bar4_Vis" 1.0 :!class /Script/Engine.MaterialInstanceDynamic)
      (Rendering|Material|SetScalarParameterValue _dmi_2 "Bar1_OY" 0.4 :!class /Script/Engine.MaterialInstanceDynamic)
      (Rendering|Material|SetScalarParameterValue _dmi_2 "Bar2_OY" 0.3 :!class /Script/Engine.MaterialInstanceDynamic)
      (Rendering|Material|SetScalarParameterValue _dmi_2 "Bar3_OY" 0.2 :!class /Script/Engine.MaterialInstanceDynamic)
      (Rendering|Material|SetScalarParameterValue _dmi_2 "Bar4_OY" 0.1 :!class /Script/Engine.MaterialInstanceDynamic)))
  (CallFunction|SetTarget 0 (Variables|Fast|GetBar1_UseHalf))
  (CallFunction|SetTarget 1 (Variables|Fast|GetBar2_UseHalf))
  (CallFunction|SetTarget 2 (Variables|Fast|GetBar3_UseHalf))
  (CallFunction|SetTarget 3 (Variables|Fast|GetBar4_UseHalf))
  (Variables|Default|SetCurrentBarIndex 0)
  (Variables|Default|SetMoverPosition 0.0)
  (Variables|Default|SetMoverDirection 1.0)
  (Rendering|Material|SetScalarParameterValue _dmi "Mover_Xpos" 0.0 :!class /Script/Engine.MaterialInstanceDynamic)
  (CallFunction|SetupMover)
  (Rendering|Material|SetScalarParameterValue _dmi "ShowActivated" 0.0 :!class /Script/Engine.MaterialInstanceDynamic)
  (Rendering|Material|SetScalarParameterValue _dmi "Bar1_Vis" 1.0 :!class /Script/Engine.MaterialInstanceDynamic)
  (Rendering|Material|SetScalarParameterValue _dmi "Bar2_Vis" 1.0 :!class /Script/Engine.MaterialInstanceDynamic)
  (Rendering|Material|SetScalarParameterValue _dmi "MoverVis" 1.0 :!class /Script/Engine.MaterialInstanceDynamic)
  (Variables|Default|SetCanMove true))

(event Custom|ReInitFailedBars
  ;[1 1 1] ReInit solved bars if current bar is failed
  (CallFunction|ReInitBar (Variables|Default|GetCurrentBarIndex))
  (if (> (Variables|Default|GetCurrentBarIndex) 0)
    (bind _output_get (Variables|Default|SetCurrentBarIndex (- (Variables|Default|GetCurrentBarIndex) 1)))
    (CallFunction|ReInitBar _output_get))
  (Variables|Default|SetMoverPosition 0.0)
  (CallFunction|SetupMover)
  (Rendering|Material|SetScalarParameterValue (Variables|Default|GetDMI) (Utilities|String|StringToName (Utilities|String|Append "Bar" (Utilities|String|ToString(Integer) (+ (Variables|Default|GetCurrentBarIndex) 1)) "_Vis")) 1.0 :!class /Script/Engine.MaterialInstanceDynamic)
  (Variables|Default|SetCanMove true))

(event Custom|ReInitBar
  (params (BarIndex :type Integer))
  ;[1 1 1] Reinit bar based on bar index
  (CallFunction|ResetBar BarIndex 0.0 0.0 (Variables|Fast|GetBarColorNormal))
  (switch int BarIndex
    (:0
      (Variables|Default|SetUseHalf (Variables|Default|GetBar1_Half)))
    (:1
      (Variables|Default|SetUseHalf (Variables|Default|GetBar2_Half)))
    (:2
      (Variables|Default|SetUseHalf (Variables|Default|GetBar3_Half)))
    (:3
      (Variables|Default|SetUseHalf (Variables|Default|GetBar4_Half))))
  (CallFunction|SetTarget BarIndex (Variables|Default|GetUseHalf)))

(event Custom|SetupMover
  (bind _currentbarindex (Variables|Default|GetCurrentBarIndex))
  (bind _dmi (Variables|Default|GetDMI))
  ;[1 1 1] Set mover postion depend on current bar index
  (Rendering|Material|SetScalarParameterValue (Variables|Default|GetDMI) "Mover_Xpos" 0.0 :!class /Script/Engine.MaterialInstanceDynamic)
  (switch Utilities|FlowControl|Switch|SwitchonE_MG_FastCount (Variables|Fast|GetBarsCount)
    (:NewEnumerator0
      (switch int _currentbarindex
        (:0
          (Rendering|Material|SetScalarParameterValue _dmi "Mover_Ypos" 0.3 :!class /Script/Engine.MaterialInstanceDynamic)
          (Variables|Default|SetMoverSpeed (Variables|Fast|GetBar1_Speed) :!label _label))
        (:1
          (Rendering|Material|SetScalarParameterValue _dmi "Mover_Ypos" 0.2 :!class /Script/Engine.MaterialInstanceDynamic)
          (Variables|Default|SetMoverSpeed (Variables|Fast|GetBar2_Speed) :!label _label_2))))
    (:NewEnumerator1
      (switch int _currentbarindex
        (:0
          (Rendering|Material|SetScalarParameterValue _dmi "Mover_Ypos" 0.35 :!class /Script/Engine.MaterialInstanceDynamic)
          (goto _label))
        (:1
          (Rendering|Material|SetScalarParameterValue _dmi "Mover_Ypos" 0.25 :!class /Script/Engine.MaterialInstanceDynamic)
          (goto _label_2))
        (:2
          (Rendering|Material|SetScalarParameterValue _dmi "Mover_Ypos" 0.15 :!class /Script/Engine.MaterialInstanceDynamic)
          (Variables|Default|SetMoverSpeed (Variables|Fast|GetBar3_Speed) :!label _label_3))))
    (:NewEnumerator2
      (switch int _currentbarindex
        (:0
          (Rendering|Material|SetScalarParameterValue _dmi "Mover_Ypos" 0.4 :!class /Script/Engine.MaterialInstanceDynamic)
          (goto _label))
        (:1
          (Rendering|Material|SetScalarParameterValue _dmi "Mover_Ypos" 0.3 :!class /Script/Engine.MaterialInstanceDynamic)
          (goto _label_2))
        (:2
          (Rendering|Material|SetScalarParameterValue _dmi "Mover_Ypos" 0.2 :!class /Script/Engine.MaterialInstanceDynamic)
          (goto _label_3))
        (:3
          (Rendering|Material|SetScalarParameterValue _dmi "Mover_Ypos" 0.1 :!class /Script/Engine.MaterialInstanceDynamic)
          (Variables|Default|SetMoverSpeed (Variables|Fast|GetBar4_Speed)))))))

(event EventBeginPlay
  ;[1 1 1] Init
  (|CallParentFunction)
  (Variables|Default|SetIsMiniGameActivated false)
  (Variables|Default|SetInputEnable false)
  (bind _returnvalue (Rendering|Material|CreateDynamicMaterialInstance "/Game/MiniGames2/Materials/MI_MiniGamesFast_Inst.MI_MiniGamesFast_Inst" "None" "None" :!class /Script/Engine.KismetMaterialLibrary))
  (Variables|Default|SetDMI _returnvalue))

(event EventTick
  (params (DeltaSeconds :type Float%20%28single-precision%29))
  ;[1 1 1] Update mover
  (|CallParentFunction DeltaSeconds)
  (if (Variables|Default|GetCanMove)
    (bind _output_get (Variables|Default|SetMoverPosition (Math|Float|Clamp(Float) (+ (Variables|Default|GetMoverPosition) (* DeltaSeconds (Variables|Default|GetMoverSpeed) (Variables|Default|GetMoverDirection))))))
    (Rendering|Material|SetScalarParameterValue (Variables|Default|GetDMI) "Mover_Xpos" _output_get :!class /Script/Engine.MaterialInstanceDynamic)
    (if (or (<= (Variables|Default|GetMoverPosition) 0.0) (>= (Variables|Default|GetMoverPosition) 1.0))
      (Variables|Default|SetMoverDirection (* (Variables|Default|GetMoverDirection) -1.0)))))

(event EventForceExit
  ;[1 1 1] Cancel
  (if (and (Variables|Default|GetMiniGameEnabled) (Variables|Default|GetIsMiniGameActivated))
    (Variables|Default|SetInputEnable false)
    (Variables|Default|SetIsMiniGameActivated false)
    (Default|CallOnMiniGameCanceled)
    (CallFunction|BlendCamerafromGametoPlayer (Variables|Default|GetOverlappedActor))))

(event EventForceAction
  (bind _returnvalue (Game|GetGameState))
  (bind _errorsound (Variables|Default|GetErrorSound))
  (bind _dmi (Variables|Default|GetDMI))
  ;[1 1 1] Button action
  (if (Variables|Default|GetPlayerOverlapped)
    (if (Variables|Default|GetIsMiniGameActivated)
      (Variables|Default|SetCanMove false)
      (switch int (Variables|Default|GetCurrentBarIndex)
        (:0
          (Variables|Default|SetTargetPos (Variables|Default|GetBar1_TargetIndex))
          (Variables|Default|SetUseHalf (Variables|Default|GetBar1_Half)))
        (:1
          (Variables|Default|SetTargetPos (Variables|Default|GetBar2_TargetIndex))
          (Variables|Default|SetUseHalf (Variables|Default|GetBar2_Half)))
        (:2
          (Variables|Default|SetTargetPos (Variables|Default|GetBar3_TargetIndex))
          (Variables|Default|SetUseHalf (Variables|Default|GetBar3_Half)))
        (:3
          (Variables|Default|SetTargetPos (Variables|Default|GetBar4_TargetIndex))
          (Variables|Default|SetUseHalf (Variables|Default|GetBar4_Half))))
      (switch int (Variables|Default|GetTargetPos)
        (:0
          (Variables|Default|SetTarget_From (Math|Float|SelectFloat (Variables|Default|GetTarget1_FromHalf) (Variables|Default|GetTarget1_From) (Variables|Default|GetUseHalf)))
          (Variables|Default|SetTarget_To (Variables|Default|GetTarget1_To)))
        (:1
          (Variables|Default|SetTarget_From (Math|Float|SelectFloat (Variables|Default|GetTarget2_FromHalf) (Variables|Default|GetTarget2_From) (Variables|Default|GetUseHalf)))
          (Variables|Default|SetTarget_To (Variables|Default|GetTarget2_To)))
        (:2
          (Variables|Default|SetTarget_From (Math|Float|SelectFloat (Variables|Default|GetTarget3_FromHalf) (Variables|Default|GetTarget3_From) (Variables|Default|GetUseHalf)))
          (Variables|Default|SetTarget_To (Variables|Default|GetTarget3_To)))
        (:3
          (Variables|Default|SetTarget_From (Math|Float|SelectFloat (Variables|Default|GetTarget4_FromHalf) (Variables|Default|GetTarget4_From) (Variables|Default|GetUseHalf)))
          (Variables|Default|SetTarget_To (Variables|Default|GetTarget4_To)))
        (:4
          (Variables|Default|SetTarget_From (Math|Float|SelectFloat (Variables|Default|GetTarget5_FromHalf) (Variables|Default|GetTarget5_From) (Variables|Default|GetUseHalf)))
          (Variables|Default|SetTarget_To (Variables|Default|GetTarget5_To)))
        (:5
          (Variables|Default|SetTarget_From (Math|Float|SelectFloat (Variables|Default|GetTarget6_FromHalf) (Variables|Default|GetTarget6_From) (Variables|Default|GetUseHalf)))
          (Variables|Default|SetTarget_To (Variables|Default|GetTarget6_To)))
        (:6
          (Variables|Default|SetTarget_From (Math|Float|SelectFloat (Variables|Default|GetTarget7_FromHalf) (Variables|Default|GetTarget7_From) (Variables|Default|GetUseHalf)))
          (Variables|Default|SetTarget_To (Variables|Default|GetTarget7_To)))
        (:7
          (Variables|Default|SetTarget_From (Variables|Default|GetTarget8_From))
          (Variables|Default|SetTarget_To (Math|Float|SelectFloat (Variables|Default|GetTarget8_ToHalf) (Variables|Default|GetTarget8_To) (Variables|Default|GetUseHalf)))))
      (if (and (>= (Variables|Default|GetMoverPosition) (Variables|Default|GetTarget_From)) (<= (Variables|Default|GetMoverPosition) (Variables|Default|GetTarget_To)))
        (bind _result (Math|Integer|IncrementInt (Variables|Default|GetCurrentBarIndex))
          (:%20%20
            (Rendering|Material|SetScalarParameterValue _dmi (Utilities|String|StringToName (Utilities|String|Append "Bar" (Utilities|String|ToString(Integer) _result) "_Vis")) 0.0 :!class /Script/Engine.MaterialInstanceDynamic)
            (if (== _result (Utilities|Select :Index (Variables|Fast|GetBarsCount) :NewEnumerator0 2 :NewEnumerator1 3 :NewEnumerator2 4))
              ;;[1 1 1] Success
              (Variables|Default|SetMiniGameEnabled false)
              (Variables|Default|SetIsMiniGameActivated false)
              (Variables|Default|SetInputEnable false)
              (Rendering|Material|SetScalarParameterValue _dmi "ShowActivated" 1.0 :!class /Script/Engine.MaterialInstanceDynamic)
              (Rendering|Material|SetScalarParameterValue _dmi "MoverVis" 0.0 :!class /Script/Engine.MaterialInstanceDynamic)
              (Utilities|FlowControl|Delay (Variables|Default|GetDelayTimeWhenComplete))
              (CallFunction|SetOfflineMaterial)
              (Default|CallOnMiniGameSuccess)
              (CallFunction|BlendCamerafromGametoPlayer (Variables|Default|GetOverlappedActor))
              (bind _research (Class|BPIPlayer|GetResearchData(Message) _returnvalue))
              (Class|BPIPlayer|SetResearchData(Message) _returnvalue (+ _research 1))
              (else
                (CallFunction|SetupMover)
                (Variables|Default|SetMoverPosition 0.0)
                (Variables|Default|SetCanMove true)))))
        (else
          ;;[1 1 1] Error
          (CallFunction|ResetBar (Variables|Default|GetCurrentBarIndex) 1.0 0.0 (Variables|Fast|GetBarColorFailed1))
          (Utilities|IsValid _errorsound
            (:Is%20Valid
              (Audio|PlaySoundatLocation _errorsound (Transformation|GetActorLocation self) "0, 0, 0" 1.0 1.0 0.0 0 0 0 0)
              (bind _newtrack_0 (Timeline|Timeline_0 PlayFromStart)
                (:Update
                  (Rendering|Material|SetVectorParameterValue (Variables|Default|GetDMI) (Utilities|String|StringToName (Utilities|String|Append "Bar" (Utilities|String|ToString(Integer) (+ (Variables|Default|GetCurrentBarIndex) 1)) "_StatusColor")) (Math|Color|Lerp(LinearColor) (Variables|Fast|GetBarColorFailed1) (Variables|Fast|GetBarColorFailed2) _newtrack_0) :!class /Script/Engine.MaterialInstanceDynamic))
                (:Finished
                  (CallFunction|ReInitFailedBars))))
            (:Is%20Not%20Valid
              (Timeline|Timeline_0 PlayFromStart)))))
      (else
        (CallFunction|InitGame)
        (Rendering|Material|SetMaterial (Variables|Default|GetMiniGameScreen) 0 (Variables|Default|GetDMI))
        (CallFunction|BlendCamerafromPlayertoGame self (Variables|Default|GetOverlappedActor))
        (Variables|Default|SetIsMiniGameActivated true)
        (Variables|Default|SetInputEnable true)))))

(fn ConstructionScript
  (|CallParentFunction))