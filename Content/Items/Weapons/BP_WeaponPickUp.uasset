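; BP_WeaponPickUp is a weapon pickup actor that gives its configured weapon to the character that interacts with it.
; ObjectInteract passes the character through a server-named RPC event to a second RPC event.
; That event calls SpawnWeapon on the character with the weapon to spawn and the pickup's location, then destroys the pickup.
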(event Custom|RPC_SpawnWeapon
  (params (Character :type BP%20Base%20Character%20Object%20Reference))
  (Default|SpawnWeapon Character (Variables|Default|GetWeaponToSpawn) (Transformation|GetActorLocation))
  (Actor|DestroyActor))

(event Custom|RPC_ServerSpawnWeapon
  (params (Character :type BP%20Base%20Character%20Object%20Reference))
  (CallFunction|RPCSpawnWeapon Character))

(event EventBeginPlay
  (|CallParentFunction) ; This node is disabled and will not be called.\nDrag off pins to build functionality.
)

(event Collision|EventActorBeginOverlap
  (params (OtherActor :type Actor%20Object%20Reference))
  (|CallParentFunction OtherActor) ; This node is disabled and will not be called.\nDrag off pins to build functionality.
)

(event EventTick
  (params (DeltaSeconds :type Float%20%28single-precision%29))
  (|CallParentFunction DeltaSeconds) ; This node is disabled and will not be called.\nDrag off pins to build functionality.
)

(event EventObjectInteract
  (params (Character :type BP%20Base%20Character%20Object%20Reference))
  (CallFunction|RPCServerSpawnWeapon Character))

(fn ConstructionScript
  (|CallParentFunction))